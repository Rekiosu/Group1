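; Base platforming ledge that can crumble after the player grabs it, then respawns.
; A grab matching this actor starts a timeline, if crumbling is enabled, that plays a sound and activates three particle systems; StopCrumble can halt it.
; On finish it hides the mesh and disables collision, releases a valid player, spawns a destructible replacement with sound, and restores itself on a respawn timer.
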(event Custom|StartCrumble
  (Audio|PlaySoundatLocation "/Game/Audio/Actual/Ledge_Start_to_crumble_sound.Ledge_Start_to_crumble_sound" (Transformation|GetActorLocation) "0, 0, 0" 1.0 1.0 0.0 0 0 0)
  (Timeline|Timeline_0 PlayFromStart
    (:Update
      (Components|Activation|Activate (Variables|Default|GetParticleSystem2) true))
    (:Finished
      (CallFunction|HideActor))))

(event Custom|StopCrumble
  (Timeline|Timeline_0 Stop
    (:Update
      (Components|Activation|Activate (Variables|Default|GetParticleSystem2) true))
    (:Finished
      (CallFunction|HideActor))))

(event EventPlayerGrabbed
  (params (ActorRef :type Actor%20Object%20Reference) (PlayerRef :type C%20Character%20Object%20Reference))
  (if (== ActorRef self)
    (Variables|Default|SetPlayerRef PlayerRef)
    (if (Variables|Default|GetCanCrumble?)
      (CallFunction|StartCrumble))))

(fn ConstructionScript)

(fn HideActor
  (bind _playerref (Variables|Default|GetPlayerRef))
  (Development|SetHiddeninGame (Variables|Default|GetStaticMesh) true false)
  (Collision|SetActorEnableCollision false)
  (Utilities|Time|SetTimerbyFunctionName 0 "UnhideActor" (Variables|Default|GetRespawnTime))
  (Utilities|IsValid _playerref
    (:Is%20Valid
      (Default|StopGrabLedge _playerref)
      (Game|SpawnActorfromClass "/Game/Blueprints/Platforming/LedgeDestructibleMesh.LedgeDestructibleMesh_C" (Transformation|GetActorTransform) "Undefined" 0 0)
      (Audio|PlaySoundatLocation "/Game/Audio/Actual/Ledge_Crumble_Sound.Ledge_Crumble_Sound" (Transformation|GetActorLocation) "0, 0, 0" 1.0 1.0 0.0 0 0 0))))

(fn UnhideActor
  (Development|SetHiddeninGame (Variables|Default|GetStaticMesh) false false)
  (Collision|SetActorEnableCollision true))