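; Butterfly actor that picks a random material for its skeletal mesh so butterflies vary in colour.
; SetColours runs from both the construction script and BeginPlay, setting slot 0 from a Materials array.
; The construction script also copies a MainMenu flag to its Butterfly_Controller, but a failed controller cast there skips the colour pick.
; An identical flag-passing chain in the event graph is unconnected.
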(event EventBeginPlay
  (CallFunction|SetColours))

(fn ConstructionScript
  (bind _asbutterfly_controller (Utilities|Casting|CastToButterfly_Controller (Pawn|GetController)))
  (Variables|/Game/Blueprints/Butterfly_Controller.Butterfly_Controller_C|SetMainMenuButterfly? _asbutterfly_controller (Variables|Default|GetMainMenu?))
  (CallFunction|SetColours))

(fn SetColours
  (bind _materials (Variables|Default|GetMaterials))
  (Rendering|Material|SetMaterial (Variables|Default|GetSkeletalMesh) 0 (Utilities|Array|Get(acopy) _materials (Math|Random|RandomInteger (Utilities|Array|Length _materials)))))