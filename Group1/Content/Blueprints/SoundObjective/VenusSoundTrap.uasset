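; VenusSoundTrap is a one-shot sound objective actor that the player triggers by entering its sphere.
; The sphere overlap checks for player character 0, then calls ActivateSound to play a sound at the actor's location.
; It then adds score to a fixed objective enum entry on the GM_Melody game mode and destroys itself, both only if that cast succeeds.
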(event OnComponentBeginOverlap(Sphere)
  (params (OverlappedComponent :type Primitive%20Component%20Object%20Reference) (OtherActor :type Actor%20Object%20Reference) (OtherComp :type Primitive%20Component%20Object%20Reference) (OtherBodyIndex :type Integer) (bFromSweep :type Boolean) (SweepResult :type Hit%20Result%20Structure%20%28by%20ref%29))
  (if (== (Game|GetPlayerCharacter 0) OtherActor)
    (CallFunction|ActivateSound)))

(event EventBeginPlay)

(event Collision|EventActorBeginOverlap
  (params (OtherActor :type Actor%20Object%20Reference)))

(event EventTick
  (params (DeltaSeconds :type Float%20%28single-precision%29)))

(fn ConstructionScript)

(fn ActivateSound
  (Audio|PlaySoundatLocation "/Game/Audio/ActivateSound.ActivateSound" (Transformation|GetActorLocation) "0, 0, 0" 1.0 1.0 0.0 0 0 0)
  (bind _asgm_melody (Utilities|Casting|CastToGM_Melody (Game|GetGameMode)))
  (Default|AddScoretoObjective _asgm_melody "NewEnumerator3")
  (Actor|DestroyActor))