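; Player controller that caches the possessed C_Character and routes movement, camera, jump, bounce and settings input to it.
; Movement is blocked when dead, stunned or hanging; forward input ramps walk speed by W hold time and enables ledge grabbing.
; Each tick it turns the mesh toward strafe input within clamped yaw limits, easing back when centered.
; The settings input replaces all widgets with the options menu and pauses the game.
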(event EventTick
  (params (DeltaSeconds :type Float%20%28single-precision%29))
  (CallFunction|LookTowardsMovement))

(event EventBeginPlay
  (CallFunction|Init))

(event Input|ActionEvents|InputActionBounce
  (params (Key :type Key%20Structure))
  (:Pressed
    (Default|BounceJump (Variables|Default|GetPlayerRef))))

(event Input|ActionEvents|InputActionSettingsInput
  (params (Key :type Key%20Structure))
  (:Pressed
    (CallFunction|SettingsUI)))

(event Input|ActionEvents|InputActionJump
  (params (Key :type Key%20Structure))
  (:Pressed
    (CallFunction|JumpCharacter)))

(event Input|AxisEvents|InputAxisForwardMovement
  (params (AxisValue :type Float%20%28single-precision%29))
  (bind _playerref (Variables|Default|GetPlayerRef))
  (bind _playerref_2 (Variables|Default|GetPlayerRef))
  (if (not (or (Variables|/Game/Blueprints/Character/C_Character.C_Character_C|GetDead _playerref) (Variables|/Game/Blueprints/Character/C_Character.C_Character_C|GetIsStunned _playerref)))
    (if (not (Variables|/Game/Blueprints/Character/C_Character.C_Character_C|GetIsHanging _playerref))
      (Pawn|Input|AddMovementInput _playerref (Transformation|GetActorForwardVector _playerref) AxisValue false)
      (if (<= AxisValue 0.1)
        (Default|ResetWalkSpeed _playerref_2)
        (Variables|/Game/Blueprints/Character/C_Character.C_Character_C|SetWantsToGrabLedge _playerref false)
        (else
          (Default|IncreaseWalkSpeed _playerref_2 (Class|PlayerController|GetInputKeyTimeDown "W"))
          (Variables|/Game/Blueprints/Character/C_Character.C_Character_C|SetWantsToGrabLedge _playerref true))))))

(event Input|AxisEvents|InputAxisRightMovement
  (params (AxisValue :type Float%20%28single-precision%29))
  (bind _playerref (Variables|Default|GetPlayerRef))
  (if (not (or (Variables|/Game/Blueprints/Character/C_Character.C_Character_C|GetDead _playerref) (Variables|/Game/Blueprints/Character/C_Character.C_Character_C|GetIsStunned _playerref)))
    (if (not (Variables|/Game/Blueprints/Character/C_Character.C_Character_C|GetIsHanging _playerref))
      (Pawn|Input|AddMovementInput _playerref (Transformation|GetActorRightVector _playerref) (select (> (Input|AxisValues|GetForwardMovement) 0.0) AxisValue (/ AxisValue 2.0)) false))))

(event Input|AxisEvents|InputAxisTurnCamera
  (params (AxisValue :type Float%20%28single-precision%29))
  (Pawn|Input|AddControllerPitchInput (Variables|Default|GetPlayerRef) (/ AxisValue 2.0)))

(event Input|AxisEvents|InputAxisLookUpCamera
  (params (AxisValue :type Float%20%28single-precision%29))
  (Pawn|Input|AddControllerYawInput (Variables|Default|GetPlayerRef) (/ AxisValue 2.0)))

(fn ConstructionScript)

(fn Init
  (Variables|Default|SetPlayerRef (.AsC%20Character (Utilities|Casting|CastToC_Character (Pawn|GetControlledPawn)))))

(fn JumpCharacter
  (bind _playerref (Variables|Default|GetPlayerRef))
  (Utilities|IsValid _playerref
    (:Is%20Valid
      (Default|StartJumping _playerref))))

(fn SettingsUI
  (bind _returnvalue (Game|GetPlayerController 0))
  (Viewport|RemoveAllWidgets)
  (bind _returnvalue_2 (UserInterface|CreateWidget "/Game/Blueprints/UI/OptionsInGame.OptionsInGame_C" _returnvalue))
  (UserInterface|Viewport|AddtoViewport _returnvalue_2 0)
  (Game|SetGamePaused true)
  (Variables|/Script/Engine.PlayerController|SetbShowMouseCursor _returnvalue true))

(fn LookTowardsMovement
  (bind _returnvalue (Input|AxisValues|GetRightMovement))
  (bind _playerref (Variables|Default|GetPlayerRef))
  (bind _playerref_2 (Variables|Default|GetPlayerRef))
  (bind _playerref_3 (Variables|Default|GetPlayerRef))
  (bind _mesh (Variables|/Script/Engine.Character|GetMesh _playerref))
  (bind _mesh_2 (Variables|/Script/Engine.Character|GetMesh _playerref_2))
  (if (not (Variables|/Game/Blueprints/Character/C_Character.C_Character_C|GetDead _playerref_3))
    (if (not (Variables|/Game/Blueprints/Character/C_Character.C_Character_C|GetIsHanging _playerref_3))
      (if (> (Input|AxisValues|GetForwardMovement) 0.0)
        (LocalVariables|SetMinRotation -1.3e+02)
        (LocalVariables|SetMaxRotation -6e+01)
        (else
          (LocalVariables|SetMinRotation -1.8e+02)
          (LocalVariables|SetMaxRotation 0.0)))
      (if (> _returnvalue 0.1)
        (Transformation|SetRelativeRotation _mesh_2 (Utilities|SwitchVariables _mesh_2 (LocalVariables|GetMinRotation) (LocalVariables|GetMaxRotation) false) false false)
        (elif (< _returnvalue -0.1)
          (Transformation|SetRelativeRotation _mesh (Utilities|SwitchVariables _mesh (LocalVariables|GetMinRotation) (LocalVariables|GetMaxRotation) true) false false)
          (elif (Math|Float|InRange(Float) _returnvalue -0.09 0.09)
            (Transformation|SetRelativeRotation _mesh (Math|Rotator|Lerp(Rotator) (Variables|/Script/Engine.SceneComponent|GetRelativeRotation _mesh) "0,-90.000000, 0" 0.1) false false)))))))