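; Player controller that handles title-screen input, the in-game HUD and toggling of the settings menu.
; The title-screen bind calls main menu creation on GM_MainMenu, while a CreationWidget event adds the in-game HUD to the viewport.
; The settings input alternates through a FlipFlop, clearing all widgets and showing either the options widget with a mouse cursor or the HUD without one.
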(event Custom|CreationWidget
  ;[1 1 1] IngameHUDCreation
  (bind _returnvalue (UserInterface|CreateWidget "/Game/Blueprints/UI/InGameHUDWidget.InGameHUDWidget_C" (Game|GetPlayerController 0)))
  (UserInterface|Viewport|AddtoViewport _returnvalue 0))

(event Input|ActionEvents|InputActionTitleScreenBind
  (params (Key :type Key%20Structure))
  ;[1 1 1] WatchForAnyInput
  (:Pressed
    (bind _asgm_mainmenu (Utilities|Casting|CastToGM_MainMenu (Game|GetGameMode)))
    (Default|MainMenuCreation _asgm_mainmenu)))

(event Input|ActionEvents|InputActionSettingsInput
  (params (Key :type Key%20Structure))
  ;[1 1 1] SettingsSwitch
  (:Pressed
    (Utilities|FlowControl|FlipFlop
      (:A
        (CallFunction|SettingsInput))
      (:B
        (CallFunction|ReturnSettingsInput)))))

(fn ConstructionScript)

(fn SettingsInput
  ;[1 1 1] DisplayingSettingsInformation
  (Viewport|RemoveAllWidgets)
  (bind _returnvalue (UserInterface|CreateWidget "/Game/Blueprints/UI/OptionsWidget.OptionsWidget_C" (Game|GetPlayerController 0)))
  (UserInterface|Viewport|AddtoViewport _returnvalue 0)
  (Variables|Default|SetbShowMouseCursor true)
  (return))

(fn ReturnSettingsInput
  ;[1 1 1] ReturnFromSettings
  (Viewport|RemoveAllWidgets)
  (bind _returnvalue (UserInterface|CreateWidget "/Game/Blueprints/UI/InGameHUDWidget.InGameHUDWidget_C" (Game|GetPlayerController 0)))
  (UserInterface|Viewport|AddtoViewport _returnvalue 0)
  (Variables|Default|SetbShowMouseCursor false)
  (return))