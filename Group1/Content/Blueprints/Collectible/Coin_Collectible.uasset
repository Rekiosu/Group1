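; Coin collectible actor that gives its static mesh a randomly chosen colored material.
; The construction script switches on a random integer to set one of the coin material instances on the first material slot.
; RandomInteger(3) only yields 0 to 2, so the silver case is never selected.
; The event graph holds only disabled placeholder events, so this Blueprint's graphs contain no pickup logic.
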(event EventBeginPlay
  (|CallParentFunction) ; This node is disabled and will not be called.\nDrag off pins to build functionality.
)

(event Collision|EventActorBeginOverlap
  (params (OtherActor :type Actor%20Object%20Reference))
  (|CallParentFunction OtherActor) ; This node is disabled and will not be called.\nDrag off pins to build functionality.
)

(event EventTick
  (params (DeltaSeconds :type Float%20%28single-precision%29))
  (|CallParentFunction DeltaSeconds) ; This node is disabled and will not be called.\nDrag off pins to build functionality.
)

(fn ConstructionScript
  (bind _staticmesh (Variables|Default|GetStaticMesh))
  (|CallParentFunction)
  (switch int (Math|Random|RandomInteger 3)
    (:0
      (Rendering|Material|SetMaterial _staticmesh 0 "/Game/Art/Materials/M_Coin_Inst_Green.M_Coin_Inst_Green"))
    (:1
      (Rendering|Material|SetMaterial _staticmesh 0 "/Game/Art/Materials/M_Coin_Inst_Orange.M_Coin_Inst_Orange"))
    (:2
      (Rendering|Material|SetMaterial _staticmesh 0 "/Game/Art/Materials/M_Coin_Inst_Purple.M_Coin_Inst_Purple"))
    (:3
      (Rendering|Material|SetMaterial _staticmesh 0 "/Game/Art/Materials/M_Coin_Inst_Silver.M_Coin_Inst_Silver"))))