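; Base collectible actor that a player character picks up by overlapping it, adding to an objective score.
; The construction script picks the static mesh from a visuals array by collectible type, either Sound Notes or Mushrooms.
; A sphere overlap casts to C_Character and calls Collect, which plays a sound, reports the type to the GM_Melody game mode, then destroys the actor.
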(event OnComponentBeginOverlap(Sphere)
  (params (OverlappedComponent :type Primitive%20Component%20Object%20Reference) (OtherActor :type Actor%20Object%20Reference) (OtherComp :type Primitive%20Component%20Object%20Reference) (OtherBodyIndex :type Integer) (bFromSweep :type Boolean) (SweepResult :type Hit%20Result%20Structure%20%28by%20ref%29))
  (CallFunction|Collect (.AsC%20Character (Utilities|Casting|CastToC_Character OtherActor))))

(event EventBeginPlay)

(event Collision|EventActorBeginOverlap
  (params (OtherActor :type Actor%20Object%20Reference)))

(event EventTick
  (params (DeltaSeconds :type Float%20%28single-precision%29)))

(fn ConstructionScript
  (bind _collectiblevisuals (Variables|Default|GetCollectibleVisuals))
  (bind _staticmesh (Variables|Default|GetStaticMesh))
  (switch Utilities|FlowControl|Switch|SwitchonObjectiveType (Variables|Default|GetTypeOfCollectible)
    (:NewEnumerator0
      (Components|StaticMesh|SetStaticMesh _staticmesh (Utilities|Array|Get(acopy) _collectiblevisuals)))
    (:NewEnumerator1
      (Components|StaticMesh|SetStaticMesh _staticmesh (Utilities|Array|Get(acopy) _collectiblevisuals 1)))))

(fn Collect
  (params (PlayerRef :type C%20Character%20Object%20Reference))
  (Utilities|IsValid PlayerRef
    (:Is%20Valid
      (Audio|PlaySound2D "/Game/Audio/ActivateSound.ActivateSound" 1.0 1.0 0.0 0 0)
      (bind _asgm_melody (Utilities|Casting|CastToGM_Melody (Game|GetGameMode)))
      (Default|AddScoretoObjective _asgm_melody (Variables|Default|GetTypeOfCollectible))
      (Actor|DestroyActor))))