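; Coin collectible variant, named for UI use, that gives its static mesh a randomly colored coin material.
; The Construction Script and BeginPlay each call the parent, then roll independently to set material slot 0, so the color can change when play begins.
; Green, orange and purple can appear; the silver branch is unreachable because the random integer's maximum is exclusive.
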(event EventBeginPlay
  (bind _staticmesh (Variables|Default|GetStaticMesh))
  (|CallParentFunction)
  (switch int (Math|Random|RandomInteger 3)
    (:0
      (Rendering|Material|SetMaterial _staticmesh 0 "/Game/Art/Materials/M_Coin_Inst_Green.M_Coin_Inst_Green"))
    (:1
      (Rendering|Material|SetMaterial _staticmesh 0 "/Game/Art/Materials/M_Coin_Inst_Orange.M_Coin_Inst_Orange"))
    (:2
      (Rendering|Material|SetMaterial _staticmesh 0 "/Game/Art/Materials/M_Coin_Inst_Purple.M_Coin_Inst_Purple"))
    (:3
      (Rendering|Material|SetMaterial _staticmesh 0 "/Game/Art/Materials/M_Coin_Inst_Silver.M_Coin_Inst_Silver"))))

(fn ConstructionScript
  (bind _staticmesh (Variables|Default|GetStaticMesh))
  (|CallParentFunction)
  (switch int (Math|Random|RandomInteger 3)
    (:0
      (Rendering|Material|SetMaterial _staticmesh 0 "/Game/Art/Materials/M_Coin_Inst_Green.M_Coin_Inst_Green"))
    (:1
      (Rendering|Material|SetMaterial _staticmesh 0 "/Game/Art/Materials/M_Coin_Inst_Orange.M_Coin_Inst_Orange"))
    (:2
      (Rendering|Material|SetMaterial _staticmesh 0 "/Game/Art/Materials/M_Coin_Inst_Purple.M_Coin_Inst_Purple"))
    (:3
      (Rendering|Material|SetMaterial _staticmesh 0 "/Game/Art/Materials/M_Coin_Inst_Silver.M_Coin_Inst_Silver"))))