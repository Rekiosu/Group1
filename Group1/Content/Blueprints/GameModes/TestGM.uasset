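; TestGM is a game mode Blueprint that manages main menu display and relays character spawn requests.
; On BeginPlay it clears all widgets through Init and shows the mouse cursor.
; MainMenuCreation clears widgets and adds a new main menu for the first player, guarded by a DoOnce that ResetMainMenu re-arms.
; CharacterSpawn forwards to CallOnCharacterSpawn, and neither it nor menu creation is triggered within this Blueprint.
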(event Custom|CharacterSpawn
  ;[1 1 1] SpawnCharacterIntoWorld
  (Default|CallOnCharacterSpawn))

(event Custom|Init
  ;[1 1 1] WidgetRemovalInitFunctionality
  (Viewport|RemoveAllWidgets))

(event Custom|MainMenuCreation
  ;[1 1 1] MainMenuWidget
  (Utilities|FlowControl|DoOnce false
    (:Completed
      (Viewport|RemoveAllWidgets)
      (bind _returnvalue (UserInterface|CreateWidget "/Game/Blueprints/UI/MainMenuWidget.MainMenuWidget_C" (Game|GetPlayerController 0)))
      (UserInterface|Viewport|AddtoViewport _returnvalue 0))))

(event Custom|ResetMainMenu
  ;[1 1 1] MainMenuWidget
  (Utilities|FlowControl|DoOnce false) ; enters at Reset
)

(event EventBeginPlay
  ;[1 1 1] EventBegin
  (CallFunction|Init)
  (Variables|/Script/Engine.PlayerController|SetbShowMouseCursor (Game|GetPlayerController 0) true))

(fn ConstructionScript)