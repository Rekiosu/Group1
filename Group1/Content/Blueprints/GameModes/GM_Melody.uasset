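; GM_Melody is a game mode that tracks collectible and enemy objectives and handles the win condition.
; On BeginPlay it creates the HUD and counts Venus sound traps, sound notes, mushrooms and enemies on the map.
; AddScoreToObjective increments the matching tally and refreshes the HUD through the character's widget reference.
; Only Venus fly traps decide victory, which clears widgets and shows YouWin; GameOver is an empty stub.
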(event EventBeginPlay
  (CallFunction|CreateHUD)
  (CallFunction|GetAllObjectivesAvailable)
  (CallFunction|GetAllEnemies))

(fn ConstructionScript)

(fn CreateHUD
  (bind _returnvalue (UserInterface|CreateWidget "/Game/Blueprints/UI/InGameHUDWidget.InGameHUDWidget_C" (Game|GetPlayerController 0)))
  (UserInterface|Viewport|AddtoViewport _returnvalue 0))

(fn GameOver
  ;[1 1 1] Just copy over to new gamemode
)

(fn CheckWinCondition
  (if (>= (Variables|Default|GetCollectedVenusFlyTraps) (Variables|Default|GetVenusFlyTrapsOnMap))
    (Development|PrintString "Win")
    (Game|SetGamePaused false)
    (Viewport|RemoveAllWidgets)
    (bind _returnvalue (UserInterface|CreateWidget "/Game/Blueprints/UI/YouWin.YouWin_C" (Game|GetPlayerController 0)))
    (UserInterface|Viewport|AddtoViewport _returnvalue 0)))

(fn AddScoretoObjective
  (params (CollectType :type ObjectiveType%20Enum :default "NewEnumerator3"))
  (switch Utilities|FlowControl|Switch|SwitchonObjectiveType CollectType
    (:NewEnumerator3
      (Variables|Default|SetCollectedVenusFlyTraps (+ (Variables|Default|GetCollectedVenusFlyTraps) 1))
      (CallFunction|UpdateHud)
      (CallFunction|CheckWinCondition))
    (:NewEnumerator0
      (Variables|Default|SetCollectedSoundNotes (+ (Variables|Default|GetCollectedSoundNotes) 1))
      (CallFunction|UpdateHud :!label _label))
    (:NewEnumerator1
      (Variables|Default|SetCollectedMushrooms (+ (Variables|Default|GetCollectedMushrooms) 1))
      (goto _label))
    (:NewEnumerator4
      (Variables|Default|SetEnemiesDefeated (+ (Variables|Default|GetEnemiesDefeated) 1))
      (goto _label))))

(fn GetAllObjectivesAvailable
  (Utilities|FlowControl|Sequence
    (:then_0
      (bind _outactors (Actor|GetAllActorsOfClass "/Game/Blueprints/SoundObjective/VenusSoundTrap.VenusSoundTrap_C"))
      (bind _output_get (Variables|Default|SetVenusFlyTrapsOnMap (Utilities|Array|Length _outactors)))
      (Development|PrintString (Utilities|String|ToString(Integer) _output_get)))
    (:then_1
      (bind _outactors_2 (Actor|GetAllActorsOfClass "/Game/Blueprints/Collectible/Coin_Collectible.Coin_Collectible_C"))
      (bind _output_get_2 (Variables|Default|SetSoundNotesOnMap (Utilities|Array|Length _outactors_2)))
      (Development|PrintString (Utilities|String|ToString(Integer) _output_get_2)))
    (:then_2
      (bind _outactors_3 (Actor|GetAllActorsOfClass "/Game/Blueprints/Collectible/Mushroom_Collectible.Mushroom_Collectible_C"))
      (bind _output_get_3 (Variables|Default|SetMushroomsOnMap (Utilities|Array|Length _outactors_3)))
      (Development|PrintString (Utilities|String|ToString(Integer) _output_get_3)))))

(fn UpdateHud
  (bind _outactors (Actor|GetAllActorsOfClass "/Game/Blueprints/Character/C_Character.C_Character_C"))
  (Utilities|IsValid (Variables|/Game/Blueprints/Character/C_Character.C_Character_C|GetInGameHUDRef (Utilities|Array|Get(acopy) _outactors))
    (:Is%20Valid
      (Default|UpdateHud (Variables|/Game/Blueprints/Character/C_Character.C_Character_C|GetInGameHUDRef (Utilities|Array|Get(acopy) _outactors))))))

(fn GetAllEnemies
  (bind _outactors (Actor|GetAllActorsOfClass "/Game/Blueprints/Enemy/AiEnemy.AiEnemy_C"))
  (Variables|Default|SetEnemyAmountOnMap (Utilities|Array|Length _outactors)))