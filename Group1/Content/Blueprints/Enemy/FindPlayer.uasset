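; Behavior tree service that finds a nearby player character for an AiEnemy pawn and stores it as the blackboard enemy.
; Each AI tick clears the Enemy key, then calls FindPlayerFunction and writes the result back if valid.
; The function runs a zero-length multi sphere trace around the pawn, ignoring itself, and casts the first hit to C_Character.
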(event EventReceiveTickAI
  (params (OwnerController :type AI%20Controller%20Object%20Reference) (ControlledPawn :type Pawn%20Object%20Reference) (DeltaSeconds :type Float%20%28single-precision%29))
  (Utilities|IsValid ControlledPawn
    (:Is%20Valid
      (Class|BTFunctionLibrary|SetBlackboardValueasObject (Variables|Default|GetEnemy))
      (bind _asai_enemy (Utilities|Casting|CastToAiEnemy ControlledPawn))
      (bind _enemy (CallFunction|FindPlayerFunction self _asai_enemy))
      (Utilities|IsValid _enemy
        (:Is%20Valid
          (Class|BTFunctionLibrary|SetBlackboardValueasObject (Variables|Default|GetEnemy) _enemy))))))

(fn FindPlayerFunction
  (params (SelfLink :type Ai%20Enemy%20Object%20Reference))
  (bind _returnvalue (Transformation|GetActorLocation SelfLink))
  (bind (_outhits _returnvalue_2) (Collision|MultiSphereTraceForObjects _returnvalue _returnvalue 5e+02 (LocalVariables|GetLocalPlayer) false (Utilities|Array|MakeArray SelfLink) "None"))
  (if _returnvalue_2
    (for _array_element _outhits
      (bind _asc_character (Utilities|Casting|CastToC_Character (.HitActor (Collision|BreakHitResult _array_element))))
      (Utilities|IsValid _asc_character
        (:Is%20Valid
          (bind _output_get (LocalVariables|SetPlayer _asc_character))
          (return _output_get))
        (:Is%20Not%20Valid
          (return (LocalVariables|GetPlayer))))))
  (return (LocalVariables|GetPlayer)))