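; Behavior tree task that turns an AiEnemy to face a location point.
; It calls Choose on the controlled enemy, then rotates its EnemyMesh to the look-at rotation toward its ChoiceOfLocationPoint.
; The rotation lerp uses a full alpha, so the mesh snaps instantly on all axes rather than turning smoothly.
; The task then finishes successfully, or aborts if the pawn is invalid or not an AiEnemy.
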(event EventReceiveExecuteAI
  (params (OwnerController :type AI%20Controller%20Object%20Reference) (ControlledPawn :type Pawn%20Object%20Reference))
  (Utilities|IsValid ControlledPawn
    (:Is%20Valid
      (bind _asai_enemy (Utilities|Casting|CastToAiEnemy ControlledPawn)
        (:then
          (Default|Choose _asai_enemy)
          (Transformation|SetWorldRotation (Variables|/Game/Blueprints/Enemy/AiEnemy.AiEnemy_C|GetEnemyMesh _asai_enemy) (Math|Rotator|MakeRotator (.roll (Math|Rotator|Lerp(Rotator) (Transformation|GetWorldRotation (Variables|/Game/Blueprints/Enemy/AiEnemy.AiEnemy_C|GetEnemyMesh _asai_enemy)) (Math|Rotator|FindLookatRotation (Transformation|GetWorldLocation (Variables|/Game/Blueprints/Enemy/AiEnemy.AiEnemy_C|GetEnemyMesh _asai_enemy)) (Transformation|GetWorldLocation (Variables|/Script/Engine.Actor|GetRootComponent (Variables|/Game/Blueprints/Enemy/AiEnemy.AiEnemy_C|GetChoiceOfLocationPoint _asai_enemy)))) 1.0)) (.pitch (Math|Rotator|Lerp(Rotator) (Transformation|GetWorldRotation (Variables|/Game/Blueprints/Enemy/AiEnemy.AiEnemy_C|GetEnemyMesh _asai_enemy)) (Math|Rotator|FindLookatRotation (Transformation|GetWorldLocation (Variables|/Game/Blueprints/Enemy/AiEnemy.AiEnemy_C|GetEnemyMesh _asai_enemy)) (Transformation|GetWorldLocation (Variables|/Script/Engine.Actor|GetRootComponent (Variables|/Game/Blueprints/Enemy/AiEnemy.AiEnemy_C|GetChoiceOfLocationPoint _asai_enemy)))) 1.0)) (.yaw (Math|Rotator|Lerp(Rotator) (Transformation|GetWorldRotation (Variables|/Game/Blueprints/Enemy/AiEnemy.AiEnemy_C|GetEnemyMesh _asai_enemy)) (Math|Rotator|FindLookatRotation (Transformation|GetWorldLocation (Variables|/Game/Blueprints/Enemy/AiEnemy.AiEnemy_C|GetEnemyMesh _asai_enemy)) (Transformation|GetWorldLocation (Variables|/Script/Engine.Actor|GetRootComponent (Variables|/Game/Blueprints/Enemy/AiEnemy.AiEnemy_C|GetChoiceOfLocationPoint _asai_enemy)))) 1.0))) false false)
          (AI|BehaviorTree|FinishExecute true))
        (:CastFailed
          (Class|BTTaskBlueprintBase|FinishAbort :!label _label))))
    (:Is%20Not%20Valid
      (goto _label))))