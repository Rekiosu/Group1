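; Behavior Tree task that makes an AiEnemy perform a charged ranged projectile attack.
; On execute it starts the charging particle and a looping timer set to the enemy's charge time.
; The timer event spawns an EnemyProjectile at the enemy's arrow, swaps particles, calls AttackColour and finishes successfully, without clearing the stored timer.
; An invalid or non-AiEnemy pawn aborts the task.
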(event Custom|Spawn
  (Utilities|IsValid (stale EventReceiveExecuteAI ControlledPawn)
    (:Is%20Valid
      (bind _asai_enemy (Utilities|Casting|CastToAiEnemy (stale EventReceiveExecuteAI ControlledPawn))
        (:then
          (Game|SpawnActorfromClass "/Game/Blueprints/Enemy/EnemyProjectile.EnemyProjectile_C" (Transformation|GetWorldTransform (Variables|/Game/Blueprints/Enemy/AiEnemy.AiEnemy_C|GetArrow1 _asai_enemy)) "Undefined" 0 (stale EventReceiveExecuteAI ControlledPawn))
          (Default|SpawnParticle _asai_enemy)
          (Components|Activation|Deactivate (Variables|/Game/Blueprints/Enemy/AiEnemy.AiEnemy_C|GetParticleSystem1 _asai_enemy))
          (Default|AttackColour _asai_enemy)
          (AI|BehaviorTree|FinishExecute true))
        (:CastFailed
          (Class|BTTaskBlueprintBase|FinishAbort :!label _label))))
    (:Is%20Not%20Valid
      (goto _label))))

(event EventReceiveExecuteAI
  (params (OwnerController :type AI%20Controller%20Object%20Reference) (ControlledPawn :type Pawn%20Object%20Reference))
  (Utilities|IsValid ControlledPawn
    (:Is%20Valid
      (bind _asai_enemy (Utilities|Casting|CastToAiEnemy ControlledPawn)
        (:then
          (Default|SpawnChargingParticle _asai_enemy)
          (bind _returnvalue (Utilities|Time|SetTimerbyEvent (delegate Custom|Spawn) (Variables|/Game/Blueprints/Enemy/AiEnemy.AiEnemy_C|GetTimeForCharge _asai_enemy) true))
          (Variables|Default|SetTimer _returnvalue))
        (:CastFailed
          (Class|BTTaskBlueprintBase|FinishAbort :!label _label))))
    (:Is%20Not%20Valid
      (goto _label))))