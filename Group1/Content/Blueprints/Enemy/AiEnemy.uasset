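; Golem enemy AI pawn that hurts the player within its damage sphere and can be squished to score an objective.
; BeginPlay gathers PointLocations with a matching ID for Choose to pick randomly, and starts looping dust puffs.
; Sphere overlap starts a looping damage timer, gated by NotHere rather than cleared.
; SquishEnemy unpossesses, flattens, scores and destroys it; glow and turning logic is disconnected.
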(event OnComponentBeginOverlap(DamageSphere)
  (params (OverlappedComponent :type Primitive%20Component%20Object%20Reference) (OtherActor :type Actor%20Object%20Reference) (OtherComp :type Primitive%20Component%20Object%20Reference) (OtherBodyIndex :type Integer) (bFromSweep :type Boolean) (SweepResult :type Hit%20Result%20Structure%20%28by%20ref%29))
  ;[1 1 1] ApplyDamage
  (Variables|Default|SetNotHere false)
  (bind _returnvalue (Utilities|Time|SetTimerbyEvent (delegate Custom|Damage) (Variables|Default|GetDamageTime) true))
  (Variables|Default|SetTimerHandle _returnvalue))

(event OnComponentEndOverlap(DamageSphere)
  (params (OverlappedComponent :type Primitive%20Component%20Object%20Reference) (OtherActor :type Actor%20Object%20Reference) (OtherComp :type Primitive%20Component%20Object%20Reference) (OtherBodyIndex :type Integer))
  ;[1 1 1] EndingVisuals
  (if (== OtherActor (Game|GetPlayerCharacter 0))
    (Variables|Default|SetNotHere true)))

(event Custom|Choose
  (bind _arrayoflocations (Variables|Default|GetArrayOfLocations))
  ;[1 1 1] LocationChoice
  (bind _output_get (Variables|Default|SetChoiceOfLocation (Math|Random|RandomInteger (Utilities|Array|Length _arrayoflocations))))
  (Variables|Default|SetChoiceOfLocationPoint (Utilities|Array|Get(acopy) _arrayoflocations _output_get)))

(event Custom|Damage
  ;[1 1 1] ApplyDamage
  (if (not (Variables|Default|GetNotHere))
    (bind _asc_character (Utilities|Casting|CastToC_Character (stale OnComponentBeginOverlap(DamageSphere) OtherActor)))
    (if (not (Variables|/Game/Blueprints/Character/C_Character.C_Character_C|GetDead _asc_character))
      (Class|DamageInterface|TakeDamage(Message) (Utilities|Array|Get(acopy) (Collision|GetOverlappingActors (Variables|Default|GetDamageSphere) "/Game/Blueprints/Character/C_Character.C_Character_C" :!class /Script/Engine.PrimitiveComponent)) (Variables|Default|GetDamagePerSecond))
      (CallFunction|SpawnParticle))))

(event Custom|AttackColour
  ;[1 1 1] SettingColours
)

(event Custom|ReturnToNormal
  ;[1 1 1] SettingColours
)

(event Custom|enemygivedust
  (Effects|SpawnEmitteratLocation "/Game/Art/Particles/P_Dust.P_Dust" (- (Transformation|GetActorLocation) "0, 0,75.000000") "0, 0, 0" "2.500000,2.500000,2.500000"))

(event Custom|SpawnParticle
  (Components|Activation|Activate (Variables|Default|GetParticleSystem) true))

(event Custom|SpawnChargingParticle
  (Components|Activation|Activate (Variables|Default|GetParticleSystem1) true))

(event EventBeginPlay
  (Utilities|Time|SetTimerbyEvent (delegate Custom|enemygivedust) 0.4 true)
  ;[1 1 1] Setup
  (Transformation|SetAbsolute (Variables|Default|GetGolem_Rocks) false true false)
  (Utilities|FlowControl|Sequence
    (:then_0
      (bind _outactors (Actor|GetAllActorsOfClass "/Game/Blueprints/Enemy/PointLocation.PointLocation_C"))
      (for _array_element _outactors
        (bind _aspoint_location (Utilities|Casting|CastToPointLocation _array_element))
        (if (== (Variables|/Game/Blueprints/Enemy/PointLocation.PointLocation_C|GetPointID _aspoint_location) (Variables|Default|GetPointIDMatch))
          (Utilities|Array|Add (Variables|Default|GetArrayOfLocations) _aspoint_location))))
    (:then_1
      (bind _output_get (Variables|Default|SetHealth (Variables|Default|GetHealth)))
      (Variables|Default|SetHealthMax _output_get)
      ;[1 1 1] StopRotation
      (Components|Movement|SetUpdatedComponent (Variables|Default|GetRotatingMovement) (Variables|Default|GetGolem_Rocks)))))

(event EventSquishEnemy
  (bind _self self)
  (bind _returnvalue (AI|GetAIController _self))
  (AI|ClearFocus _returnvalue)
  (Pawn|UnPossess _returnvalue)
  (Transformation|SetWorldRotation (Variables|Default|GetGolem_Rocks) (Variables|Default|GetStartRot) false false)
  (Transformation|SetWorldScale3D (Variables|Default|GetEnemyMesh) "1.000000,1.000000,0.100000")
  (bind _asgm_melody (Utilities|Casting|CastToGM_Melody (Game|GetGameMode)))
  (Default|AddScoretoObjective _asgm_melody "NewEnumerator4")
  (Utilities|FlowControl|Delay 1.0)
  (Actor|DestroyActor))

(event EventTick
  (params (DeltaSeconds :type Float%20%28single-precision%29)))

(fn ConstructionScript)