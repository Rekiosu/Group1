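; Behavior tree node for AiEnemy pawns that flags whether a C_Character is within range.
; On each AI tick it runs a zero-length sphere trace at the pawn's location as a radius overlap check, ignoring the pawn itself.
; It sets the IsAtEnemyLocation blackboard bool true if the single returned hit is a C_Character, and false on any other hit or none.
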(event EventReceiveTickAI
  (params (OwnerController :type AI%20Controller%20Object%20Reference) (ControlledPawn :type Pawn%20Object%20Reference) (DeltaSeconds :type Float%20%28single-precision%29))
  (bind _isatenemylocation (Variables|Default|GetIsAtEnemyLocation))
  (Utilities|IsValid ControlledPawn
    (:Is%20Valid
      (bind _asai_enemy (Utilities|Casting|CastToAiEnemy ControlledPawn))
      (bind (_outhit _returnvalue) (Collision|SphereTraceForObjects (Transformation|GetActorLocation _asai_enemy) (Transformation|GetActorLocation _asai_enemy) 526.0 (Variables|Default|GetNewVar_1) false (Utilities|Array|MakeArray _asai_enemy) "None"))
      (if _returnvalue
        (Utilities|Casting|CastToC_Character (.HitActor (Collision|BreakHitResult _outhit))
          (:then
            (Class|BTFunctionLibrary|SetBlackboardValueasBool _isatenemylocation true))
          (:CastFailed
            (Class|BTFunctionLibrary|SetBlackboardValueasBool _isatenemylocation false :!label _label)))
        (else
          (goto _label))))))