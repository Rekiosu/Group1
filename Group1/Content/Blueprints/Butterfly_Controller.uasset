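; AI controller that makes a butterfly wander around its starting location.
; On BeginPlay it gives the pawn a random scale, caches the level's nav meshes and records the start position.
; MoveTo sends the pawn to random navigable points within a radius of that origin, re-calling itself on success or failure.
; The UpAndDown timeline adds a world offset to the pawn on each update, layering bobbing motion over the movement.
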(event Custom|MoveTo
  (AI|AIMoveTo (Pawn|GetControlledPawn) (.RandomLocation (Class|NavigationSystemV1|GetRandomPointinNavigableRadius (Variables|Default|GetInitialLocaiton) (Variables|Default|GetRadiusSize) (Utilities|Array|Get(acopy) (Variables|Default|GetNavMesh)) "/Script/AIModule.NavFilter_AIControllerDefault")) 0 1e+02 false
    (:OnSuccess
      _)
    (:OnFail
      _))
  (CallFunction|Moveto))

(event EventBeginPlay
  (Transformation|SetActorScale3D (Pawn|GetControlledPawn) (Math|Conversions|ToVector(Float) (Math|Random|RandomFloatinRange 2.0 4.0)))
  (bind _outactors (Actor|GetAllActorsOfClass "/Script/NavigationSystem.RecastNavMesh"))
  (Variables|Default|SetNavMesh _outactors)
  (Variables|Default|SetInitialLocaiton (Transformation|GetActorLocation (Pawn|GetControlledPawn)))
  (CallFunction|Moveto)
  (bind _newtrack_0 (Timeline|UpAndDown PlayFromStart)
    (:Update
      (Transformation|AddActorWorldOffset (Pawn|GetControlledPawn) _newtrack_0))))

(fn ConstructionScript)