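; Platformer character with double jump, ledge grab and climb, and a bounce slam that squishes enemies or stuns the character on other surfaces.
; Tick drives speed-based camera lag and distance, forward and height traces for ledge grabs, HUD health flashes, and lagged position feeds to grass material parameters.
; A timeline capsule-traces during slams.
; Looping timers regenerate health after damage and record recent ground checkpoints, choosing pawn-free ones for respawn.
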(event Custom|GrabLedge
  (params (ActorGrabbing :type Actor%20Object%20Reference))
  (bind (_vector _rotation) (Utilities|LedgePointCalculation))
  ;[1 1 1] Grab the Ledge
  (Utilities|CheckCanGrab)
  (Pawn|Components|CharacterMovement|SetMovementMode (Variables|Character|GetCharacterMovement) "MOVE_Flying" 0)
  (Variables|WallClimbing|SetIsHanging true)
  (Components|MoveComponentTo (Variables|Collision|GetCapsuleComponent) _vector _rotation false false 0.2 false)
  (Components|Movement|StopMovementImmediately (Variables|Character|GetCharacterMovement))
  (WallClimbing|DisableRotBasedfromCamera)
  (CallFunction|StopBounceJump)
  (Variables|WallClimbing|SetJustHanged true)
  (Utilities|Time|SetTimerbyFunctionName 0 "ClearJustHanged" (Variables|WallClimbing|GetWallHangCooldown))
  (Camera|SeperateCameraRotationfromPlayer))

(event Custom|ClimbLedge
  ;[0 1 0.1589] Climb Ledge
  (if (not (Variables|WallClimbing|GetIsClimbingLedge))
    (Character|LaunchCharacter (Math|Vector|MakeVector 0.0 0.0 7.5e+02) false true)
    (Pawn|Components|CharacterMovement|SetMovementMode (Variables|Character|GetCharacterMovement) "MOVE_Walking" 0)
    (Variables|WallClimbing|SetIsClimbingLedge true)
    (Variables|WallClimbing|SetIsHanging false)
    (Utilities|FlowControl|Delay 0.2)
    (Variables|WallClimbing|SetIsClimbingLedge false)
    (WallClimbing|RenableRotBasedfromCamera)
    (CallFunction|StopBounceJump)
    (Camera|CombineCameraRotationtoPlayer)))

(event Custom|CallBounceEFfect
  (CallFunction|BounceEffect (stale EventBounceCharacter BounceAmount)))

(event Custom|StopBounceJump
  (bind _returnvalue (Transformation|GetActorLocation))
  (bind _returnvalue_2 (Transformation|GetActorLocation))
  ;[1 1 1] Bounce Jumping
  (Variables|Jumping|SetIsBouncing false)
  (Variables|/Script/Engine.CharacterMovementComponent|SetGravityScale (Variables|Character|GetCharacterMovement) 1.0)
  (Timeline|Timeline_0 Stop
    (:Update
      (bind (_outhit _returnvalue_3) (Collision|CapsuleTraceByChannel _returnvalue (- _returnvalue "0, 0,115.000000") 65.0 88.0 "TraceTypeQuery4" false (Utilities|Array|MakeArray self) "ForOneFrame"))
      (if (Variables|Jumping|GetIsBouncing)
        (if _returnvalue_3
          (if (Utilities|DoesObjectImplementInterface (.HitActor (Collision|BreakHitResult _outhit)) "/Game/Blueprints/Interface/DamageInterface.DamageInterface_C")
            (Class|DamageInterface|SquishEnemy(Message) (.HitActor (Collision|BreakHitResult _outhit))))
          (Animation|PlayAnimMontage "/Game/Art/Animations/NewMelodyCharacter/MelodyMontage.MelodyMontage" 1.0 "BounceAction")
          (CallFunction|StopBounceTime)
          (else
            (bind _returnvalue_4 (Collision|CapsuleTraceByChannel _returnvalue_2 (- _returnvalue_2 "0, 0,125.000000") 65.0 88.0 "TraceTypeQuery1" false (Utilities|Array|MakeArray self) "ForOneFrame"))
            (if _returnvalue_4
              (Health|Stunned))))
        (else
          (CallFunction|StopBounceJump))))))

(event Custom|StopGrabLedge
  (Pawn|Components|CharacterMovement|SetMovementMode (Variables|Character|GetCharacterMovement) "MOVE_Walking" 0)
  (Variables|WallClimbing|SetIsHanging false)
  (Utilities|FlowControl|Delay 0.2)
  (WallClimbing|RenableRotBasedfromCamera)
  (CallFunction|StopBounceJump)
  (Camera|CombineCameraRotationtoPlayer))

(event Custom|StopBounceTime
  (bind _returnvalue (Transformation|GetActorLocation))
  (bind _returnvalue_2 (Transformation|GetActorLocation))
  ;[1 1 1] Bounce Jumping
  (Timeline|Timeline_0 Stop
    (:Update
      (bind (_outhit _returnvalue_3) (Collision|CapsuleTraceByChannel _returnvalue (- _returnvalue "0, 0,115.000000") 65.0 88.0 "TraceTypeQuery4" false (Utilities|Array|MakeArray self) "ForOneFrame"))
      (if (Variables|Jumping|GetIsBouncing)
        (if _returnvalue_3
          (if (Utilities|DoesObjectImplementInterface (.HitActor (Collision|BreakHitResult _outhit)) "/Game/Blueprints/Interface/DamageInterface.DamageInterface_C")
            (Class|DamageInterface|SquishEnemy(Message) (.HitActor (Collision|BreakHitResult _outhit))))
          (Animation|PlayAnimMontage "/Game/Art/Animations/NewMelodyCharacter/MelodyMontage.MelodyMontage" 1.0 "BounceAction")
          (CallFunction|StopBounceTime)
          (else
            (bind _returnvalue_4 (Collision|CapsuleTraceByChannel _returnvalue_2 (- _returnvalue_2 "0, 0,125.000000") 65.0 88.0 "TraceTypeQuery1" false (Utilities|Array|MakeArray self) "ForOneFrame"))
            (if _returnvalue_4
              (Health|Stunned))))
        (else
          (CallFunction|StopBounceJump))))))

(event Custom|StartBounce
  (bind _returnvalue (Transformation|GetActorLocation))
  (bind _returnvalue_2 (Transformation|GetActorLocation))
  (bind _charactermovement (Variables|Character|GetCharacterMovement))
  ;[1 1 1] Bounce Jumping
  (Variables|/Script/Engine.CharacterMovementComponent|SetGravityScale _charactermovement 2.0)
  (Pawn|Components|CharacterMovement|SetMovementMode _charactermovement "MOVE_Falling" 0)
  (Character|LaunchCharacter "0, 0,-750.000000" false true)
  (Timeline|Timeline_0 Play
    (:Update
      (bind (_outhit _returnvalue_3) (Collision|CapsuleTraceByChannel _returnvalue (- _returnvalue "0, 0,115.000000") 65.0 88.0 "TraceTypeQuery4" false (Utilities|Array|MakeArray self) "ForOneFrame"))
      (if (Variables|Jumping|GetIsBouncing)
        (if _returnvalue_3
          (if (Utilities|DoesObjectImplementInterface (.HitActor (Collision|BreakHitResult _outhit)) "/Game/Blueprints/Interface/DamageInterface.DamageInterface_C")
            (Class|DamageInterface|SquishEnemy(Message) (.HitActor (Collision|BreakHitResult _outhit))))
          (Animation|PlayAnimMontage "/Game/Art/Animations/NewMelodyCharacter/MelodyMontage.MelodyMontage" 1.0 "BounceAction")
          (CallFunction|StopBounceTime)
          (else
            (bind _returnvalue_4 (Collision|CapsuleTraceByChannel _returnvalue_2 (- _returnvalue_2 "0, 0,125.000000") 65.0 88.0 "TraceTypeQuery1" false (Utilities|Array|MakeArray self) "ForOneFrame"))
            (if _returnvalue_4
              (Health|Stunned))))
        (else
          (CallFunction|StopBounceJump))))))

(event Custom|BounceEffect
  (params (BounceAmount :type Float%20%28single-precision%29))
  (Effects|SpawnEmitteratLocation "/Game/Art/Particles/P_SmokeRing.P_SmokeRing" (- (.location (Transformation|GetActorTransform)) "0, 0,45.000000"))
  (Character|LaunchCharacter (Math|Vector|MakeVector 0.0 0.0 (* BounceAmount 1.52)) false true)
  (Audio|PlaySoundatLocation "/Game/Audio/Actual/Bounce.Bounce" (Transformation|GetActorLocation) "0, 0, 0" 1.0 1.0 0.0 0 0 0)
  (Variables|Jumping|SetHasJustBounced true)
  (CallFunction|StopBounceJump))

(event EventAllowBounceJump
  (Variables|Jumping|SetCanBounce true))

(event EventTick
  (params (DeltaSeconds :type Float%20%28single-precision%29))
  ;[0 1 0.09635] Low performance cost
  (Camera|CameraSettings)
  (WallClimbing|TraceForward)
  (WallClimbing|TraceDistancefromGround)
  ;[1 0.8213 0] Its fine but if anymore stufflike this gets added it will start to tank FPS
  (CallFunction|UpdateGrass)
  ;[1 1 1] HealthIncreaseVisual
  (Health|HealthIncreaseVisual)
  (CallFunction|Updateclouds))

(event EventTakeDamage
  (params (Damage :type Float%20%28single-precision%29))
  ;[0.2661 1 0] Damage
  (Health|ReduceHealth Damage))

(event EventOnLanded
  (params (Hit :type Hit%20Result%20Structure%20%28by%20ref%29))
  (Jumping|LandEvent))

(event EventAllowAnotherJump
  (Jumping|ResetDoubleJump))

(event EventBounceCharacter
  (params (Instant? :type Boolean) (BounceAmount :type Float%20%28single-precision%29))
  (if Instant?
    (CallFunction|BounceEffect BounceAmount)
    (else
      (Utilities|Time|SetTimerbyEvent (delegate Custom|CallBounceEFfect) 0.15))))

(event EventBeginPlay
  (CallFunction|InitCheckpoint))

(fn ConstructionScript)

(fn StartJumping
  (bind _charactermovement (Variables|Character|GetCharacterMovement))
  (bind _jumpzvelocity (Variables|/Script/Engine.CharacterMovementComponent|GetJumpZVelocity _charactermovement))
  (if (Variables|WallClimbing|GetIsHanging)
    (CallFunction|ClimbLedge)
    (elif (AI|Components|NavMovement|IsFalling (Variables|Character|GetCharacterMovement))
      (if (Variables|Jumping|GetCanDoubleJump)
        (Animation|PlayAnimMontage "/Game/Art/Animations/NewMelodyCharacter/MelodyMontage.MelodyMontage" 1.0 "Jump")
        (Character|LaunchCharacter (Math|Vector|MakeVector 0.0 0.0 (* _jumpzvelocity (LocalVariables|GetSecondJumpHeightMultiplier))) false true)
        (Variables|Jumping|SetCanDoubleJump false)
        (Audio|PlaySoundatLocation "/Game/Audio/DoubleJump.DoubleJump" (Transformation|GetActorLocation) "0, 0, 0" 1.0 1.0 0.0 0 0 0)
        (Variables|Jumping|SetCanBounce (select (Variables|Jumping|GetHasJustBounced) false true))
        (Effects|SpawnEmitteratLocation "/Game/Art/Particles/P_DoubleJump.P_DoubleJump" (Transformation|GetActorLocation) "0, 0, 0" "3.000000,3.000000,3.000000")
        (Utilities|Time|SetTimerbyFunctionName 0 "ResetJumpedVariable" 0.2 :!label _label))
      (else
        (Animation|PlayAnimMontage "/Game/Art/Animations/NewMelodyCharacter/MelodyMontage.MelodyMontage" 1.0 "Jump")
        (Character|LaunchCharacter (Math|Vector|MakeVector 0.0 0.0 (* _jumpzvelocity (LocalVariables|GetFirstJumpHeightMultiplier))) false false)
        (Audio|PlaySoundatLocation "/Game/Audio/IntialJump.IntialJump" (Transformation|GetActorLocation) "0, 0, 0" 1.0 1.0 0.0 0 0 0)
        (Variables|Jumping|SetJumped_Anim true)
        (goto _label)))))

(fn ResetDoubleJump
  (Variables|Jumping|SetCanDoubleJump true))

(fn CameraSettings
  (bind _springarm (Variables|Default|GetSpringArm))
  (if (> (Math|Vector|VectorLength (Variables|/Script/Engine.MovementComponent|GetVelocity (Variables|Character|GetCharacterMovement))) 4e+02)
    ;[1 1 1] Slow
    (Variables|/Script/Engine.SpringArmComponent|SetCameraLagSpeed _springarm (Math|Float|Lerp (Variables|/Script/Engine.SpringArmComponent|GetCameraLagSpeed _springarm) 5.0 0.5))
    (Variables|/Script/Engine.SpringArmComponent|SetTargetArmLength _springarm (Math|Float|Lerp (Variables|/Script/Engine.SpringArmComponent|GetTargetArmLength _springarm) 1.25e+03 0.005))
    (else
      ;[1 1 1] Fast
      (Variables|/Script/Engine.SpringArmComponent|SetCameraLagSpeed _springarm (Math|Float|Lerp (Variables|/Script/Engine.SpringArmComponent|GetCameraLagSpeed _springarm) 1e+01 0.5))
      (Variables|/Script/Engine.SpringArmComponent|SetTargetArmLength _springarm (Math|Float|Lerp (Variables|/Script/Engine.SpringArmComponent|GetTargetArmLength _springarm) 7.5e+02 0.01)))))

(fn TraceForward
  (bind _returnvalue (Transformation|GetActorLocation))
  (bind _returnvalue_2 (Transformation|GetActorRotation))
  (bind _returnvalue_3 (Math|Vector|GetForwardVector _returnvalue_2))
  (if (not (Variables|WallClimbing|GetIsHanging))
    (bind (_outhit _returnvalue_4) (Collision|SphereTraceByChannel _returnvalue (+ _returnvalue (Math|Vector|MakeVector (* (.x _returnvalue_3) 1.5e+02) (* (.y _returnvalue_3) 1.5e+02) (.z _returnvalue_3))) 2e+01 "TraceTypeQuery3" false (Utilities|Array|MakeArray self) "None"))
    (if _returnvalue_4
      (Variables|WallClimbing|SetWallLocation (.Location (Collision|BreakHitResult _outhit)))
      (Variables|WallClimbing|SetWallNormal (.Normal (Collision|BreakHitResult _outhit)))
      (Variables|Default|SetTraceForwardActorRef (.HitActor (Collision|BreakHitResult _outhit))))))

(fn TraceDistancefromGround
  (bind _returnvalue (Transformation|GetActorLocation))
  (bind _returnvalue_2 (Transformation|GetActorRotation))
  (bind _traceforwardactorref (Variables|Default|GetTraceForwardActorRef))
  (bind _returnvalue_3 (Math|Vector|GetForwardVector _returnvalue_2))
  (bind _returnvalue_4 (+ (.z _returnvalue) 5e+02))
  (bind _returnvalue_5 (* _returnvalue_3 7e+01))
  (bind _returnvalue_6 (Math|Vector|MakeVector (.x _returnvalue) (.y _returnvalue) _returnvalue_4))
  (bind _returnvalue_7 (+ _returnvalue_6 _returnvalue_5))
  (bind (_x _y _z) (Math|Vector|BreakVector _returnvalue_7))
  (if (not (Variables|WallClimbing|GetIsHanging))
    (bind (_outhit _returnvalue_8) (Collision|SphereTraceByChannel _returnvalue_7 (Math|Vector|MakeVector _x _y (- _z 5e+02)) 2e+01 "TraceTypeQuery3" false (Utilities|Array|MakeArray self) "None"))
    (if _returnvalue_8
      (LocalVariables|SetStartRotation (Transformation|GetWorldRotation (Variables|Collision|GetCapsuleComponent)))
      (Variables|WallClimbing|SetHeightLocation (.Location (Collision|BreakHitResult _outhit)))
      (if (Math|Float|InRange(Float) (- (.z (Transformation|GetWorldLocation (Variables|Default|GetBillboard))) (.Z (Math|Vector|BreakVector (Variables|WallClimbing|GetHeightLocation)))) -2e+02 0.0)
        (if (not (Variables|WallClimbing|GetIsClimbingLedge))
          (Utilities|IsValid _traceforwardactorref
            (:Is%20Valid
              (CallFunction|GrabLedge _traceforwardactorref))))))))

(fn DisableRotBasedfromCamera)

(fn RenableRotBasedfromCamera)

(fn IncreaseWalkSpeed
  (params (KeyHoldTime :type Float%20%28single-precision%29))
  (bind _charactermovement (Variables|Character|GetCharacterMovement))
  (Variables|/Script/Engine.CharacterMovementComponent|SetMaxWalkSpeed _charactermovement (Math|Float|Clamp(Float) (+ (Variables|/Script/Engine.CharacterMovementComponent|GetMaxWalkSpeed _charactermovement) (* (Variables|WalkSpeeds|GetWalkSpeedIncreaseAmount) KeyHoldTime)) (Variables|WalkSpeeds|GetInitialWalkSpeed) (Variables|WalkSpeeds|GetMaxWalkSpeed))))

(fn ResetWalkSpeed
  (if (not (Variables|WallClimbing|GetIsHanging))
    (Variables|/Script/Engine.CharacterMovementComponent|SetMaxWalkSpeed (Variables|Character|GetCharacterMovement) (Variables|WalkSpeeds|GetInitialWalkSpeed))))

(fn LandEvent
  (if (Variables|Jumping|GetHasJustBounced)
    _
    (else
      (Jumping|ResetDoubleJump)
      (Audio|PlaySoundatLocation "/Game/Audio/Land.Land" (Transformation|GetActorLocation) "0, 0, 0" 1.0 1.0 0.0 0 0 0)))
  (CallFunction|StopBounceJump)
  (Variables|Jumping|SetHasJustBounced false))

(fn ClearJustHanged
  (Variables|WallClimbing|SetJustHanged false))

(fn TraceforCheckpoint
  (bind _returnvalue (Transformation|GetActorLocation))
  (bind _previouscheckpoints (Variables|Default|GetPreviousCheckpoints))
  (if (not (Math|Boolean|ORBoolean (AI|Components|NavMovement|IsFalling (Variables|Character|GetCharacterMovement)) (Variables|WallClimbing|GetIsHanging) (Variables|WallClimbing|GetIsClimbingLedge) (Variables|Jumping|GetIsBouncing)))
    (bind (_outhit _returnvalue_2) (Collision|LineTraceByChannel _returnvalue (- _returnvalue "0, 0,115.000000") "TraceTypeQuery5" false (Utilities|Array|MakeArray self) "None"))
    (if _returnvalue_2
      (Utilities|Array|AddUnique _previouscheckpoints (.Location (Collision|BreakHitResult _outhit))))
    (if (>= (Utilities|Array|Length _previouscheckpoints) 3)
      (Utilities|Array|RemoveIndex _previouscheckpoints))
    (for _array_element _previouscheckpoints
      (bind _returnvalue_3 (Collision|SphereTraceForObjects _array_element _array_element 2.5e+02 (Utilities|Array|MakeArray "ObjectTypeQuery3") false (Utilities|Array|MakeArray self) "None"))
      (if (not _returnvalue_3)
        (Variables|Default|SetRespawnLoc _array_element)))))

(fn ReduceHealth
  (params (HealthReduction :type Float%20%28single-precision%29))
  (Variables|Default|SetHealth (- (Variables|Default|GetHealth) HealthReduction))
  (bind _returnvalue (Utilities|Time|SetTimerbyFunctionName 0 "RegenHealth" 1.0 true))
  (Variables|Default|SetHealthRegen _returnvalue)
  (Health|HealthDecreaseVisual)
  (Camera|PlayWorldCameraShake "/Game/Blueprints/CameraShakes/PlayerHit.PlayerHit_C" (Transformation|GetActorLocation) 1.0 1.25e+03)
  (if (<= (Variables|Default|GetHealth) 0.0)
    (Health|RespawnatLastCheckpoint)
    (elif (<= (Variables|Default|GetHealth) 75.0)
      (Default|HealthFlashStart (Variables|References|GetInGameHUDRef))
      (if (<= (Variables|Default|GetHealth) 5e+01)
        (Default|MediumHealthFlash (Variables|References|GetInGameHUDRef))
        (if (<= (Variables|Default|GetHealth) 25.0)
          (Default|MaxHealthFlash (Variables|References|GetInGameHUDRef))))
      (else
        (Default|StopAnimation (Variables|References|GetInGameHUDRef))))))

(fn RespawnatLastCheckpoint
  (CallFunction|StopBounceJump)
  (Variables|Default|SetbUseControllerRotationYaw false)
  (Variables|Default|SetDead true)
  (Transformation|SetActorLocation (+ (Variables|Default|GetRespawnLoc) "0, 0,35.000000") false false)
  (Components|Movement|StopMovementImmediately (Variables|Character|GetCharacterMovement))
  (Default|StopAnimation (Variables|References|GetInGameHUDRef))
  (Variables|Default|SetHealth (Variables|Default|GetHealthMax))
  (Animation|PlayAnimMontage "/Game/Art/Animations/NewMelodyCharacter/MelodyMontage.MelodyMontage" 1.0 "Revive"))

(fn SeperateCameraRotationfromPlayer
  (Variables|Default|SetbUseControllerRotationYaw false))

(fn CombineCameraRotationtoPlayer
  (Variables|Default|SetbUseControllerRotationYaw true))

(fn UpdateGrass
  (bind _returnvalue (Transformation|GetActorLocation))
  (Rendering|Material|SetVectorParameterValue "/Game/Art/GrassParams.GrassParams" "PlayerPos" (Math|Conversions|ToLinearColor(Vector) _returnvalue) :!class /Script/Engine.KismetMaterialLibrary)
  (bind _output_get (LocalVariables|SetP2 (Math|Vector|Lerp(Vector) (LocalVariables|GetP2) _returnvalue 0.005)))
  (Rendering|Material|SetVectorParameterValue "/Game/Art/GrassParams.GrassParams" "P2" (Math|Conversions|ToLinearColor(Vector) _output_get) :!class /Script/Engine.KismetMaterialLibrary)
  (bind _output_get_2 (LocalVariables|SetP3 (Math|Vector|Lerp(Vector) (LocalVariables|GetP3) _returnvalue 0.001)))
  (Rendering|Material|SetVectorParameterValue "/Game/Art/GrassParams.GrassParams" "P3" (Math|Conversions|ToLinearColor(Vector) _output_get_2) :!class /Script/Engine.KismetMaterialLibrary))

(fn HealthDecreaseVisual
  (if (<= (Variables|Default|GetHealth) 75.0)
    (Default|HealthFlashStart (Variables|References|GetInGameHUDRef))
    (if (<= (Variables|Default|GetHealth) 5e+01)
      (Default|MediumHealthFlash (Variables|References|GetInGameHUDRef))
      (if (<= (Variables|Default|GetHealth) 25.0)
        (Default|MaxHealthFlash (Variables|References|GetInGameHUDRef))
        (return)
        (else
          (return)))
      (else
        (return)))
    (else
      (Default|StopAnimation (Variables|References|GetInGameHUDRef))
      (return))))

(fn HealthIncreaseVisual
  (Utilities|IsValid (Variables|References|GetInGameHUDRef)
    (:Is%20Valid
      (if (>= (Variables|Default|GetHealth) 1e+02)
        (Variables|Default|SetHealth 1e+02)
        (Default|StopAnimation (Variables|References|GetInGameHUDRef))
        (elif (>= (Variables|Default|GetHealth) 8e+01)
          (Default|StopAnimation (Variables|References|GetInGameHUDRef))
          (elif (>= (Variables|Default|GetHealth) 6e+01)
            (Default|LowHealthFlash (Variables|References|GetInGameHUDRef))
            (return)
            (elif (>= (Variables|Default|GetHealth) 3e+01)
              (Default|MediumHealthFlash (Variables|References|GetInGameHUDRef))
              (return)
              (else
                (return))))))
      (return))))

(fn ResetJumpedVariable
  (Variables|Jumping|SetJumped_Anim false))

(fn Updateclouds)

(fn HeightCheckforBounce)

(fn ResetDead
  (Variables|Default|SetDead false)
  (Variables|Default|SetbUseControllerRotationYaw true))

(fn BounceJump
  (bind _charactermovement (Variables|Character|GetCharacterMovement))
  (if (not (Variables|Default|GetDead))
    (if (Variables|Jumping|GetCanBounce)
      (Animation|PlayAnimMontage "/Game/Art/Animations/NewMelodyCharacter/MelodyMontage.MelodyMontage" 1.0 "BounceFallStart")
      (Variables|Jumping|SetIsBouncing true)
      (Variables|Jumping|SetCanBounce false)
      (Components|Movement|StopMovementImmediately _charactermovement)
      (Pawn|Components|CharacterMovement|SetMovementMode _charactermovement "MOVE_Flying" 0)
      (Character|LaunchCharacter "0, 0,500.000000" false true))))

(fn Stunned
  (Components|Movement|StopMovementImmediately (Variables|Character|GetCharacterMovement))
  (Variables|Default|SetIsStunned true)
  (CallFunction|StopBounceJump)
  (Variables|Default|SetbUseControllerRotationYaw false)
  (Default|StopAnimation (Variables|References|GetInGameHUDRef))
  (Animation|PlayAnimMontage "/Game/Art/Animations/NewMelodyCharacter/MelodyMontage.MelodyMontage" 1.0 "Stunned")
  (Camera|PlayWorldCameraShake "/Game/Blueprints/CameraShakes/Stunned.Stunned_C" (Transformation|GetActorLocation) 3e+03 3e+03))

(fn ResetStunned
  (Variables|Default|SetIsStunned false)
  (Variables|Default|SetbUseControllerRotationYaw true))

(fn RegenHealth
  (bind _healthmax (Variables|Default|GetHealthMax))
  (if (== (Variables|Default|GetHealth) _healthmax)
    (Utilities|Time|ClearandInvalidateTimerbyHandle (Variables|Default|GetHealthRegen))
    (else
      (Variables|Default|SetHealth (Math|Float|Clamp(Float) (+ (Variables|Default|GetHealth) 5.0) 0.0 _healthmax))
      (Health|HealthIncreaseVisual))))

(fn InitCheckpoint
  (bind _returnvalue (Utilities|Time|SetTimerbyFunctionName 0 "TraceForCheckpoint" 1.0 true))
  (Variables|Default|SetCheckpointTraceTimer _returnvalue)
  (Utilities|Array|Resize (Variables|Default|GetPreviousCheckpoints) 3))