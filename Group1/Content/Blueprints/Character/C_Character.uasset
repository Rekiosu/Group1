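; Player character Blueprint that adds a sound-backed double jump and speed-sensitive camera lag.
; StartJumping does a normal jump when grounded or one boosted launch while falling, gated by CanDoubleJump.
; Landing or the AllowAnotherJump event restores that flag.
; Each tick, spring arm lag speed eases toward one value when moving fast on the ground and toward zero when falling or slow.
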(event EventBeginPlay)

(event Collision|EventActorBeginOverlap
  (params (OtherActor :type Actor%20Object%20Reference)))

(event EventTick
  (params (DeltaSeconds :type Float%20%28single-precision%29))
  (CallFunction|CameraSettings DeltaSeconds))

(event EventOnLanded
  (params (Hit :type Hit%20Result%20Structure%20%28by%20ref%29))
  (CallFunction|ResetDoubleJump)
  (Audio|PlaySoundatLocation "/Game/Audio/Land.Land" (Transformation|GetActorLocation) "0, 0, 0" 1.0 1.0 0.0 0 0 0))

(event EventAllowAnotherJump
  (CallFunction|ResetDoubleJump))

(fn ConstructionScript)

(fn StartJumping
  (if (AI|Components|NavMovement|IsFalling (Variables|Character|GetCharacterMovement))
    (if (Variables|Default|GetCanDoubleJump)
      (Character|LaunchCharacter (Math|Vector|MakeVector 0.0 0.0 (* (Variables|/Script/Engine.CharacterMovementComponent|GetJumpZVelocity (Variables|Character|GetCharacterMovement)) 1.5)) false false)
      (Variables|Default|SetCanDoubleJump false)
      (Audio|PlaySoundatLocation "/Game/Audio/DoubleJump.DoubleJump" (Transformation|GetActorLocation) "0, 0, 0" 1.0 1.0 0.0 0 0 0))
    (else
      (Character|Jump)
      (Audio|PlaySoundatLocation "/Game/Audio/IntialJump.IntialJump" (Transformation|GetActorLocation) "0, 0, 0" 1.0 1.0 0.0 0 0 0))))

(fn ResetDoubleJump
  (Variables|Default|SetCanDoubleJump true))

(fn CameraSettings
  (params (Delta :type Float%20%28single-precision%29))
  (bind _charactermovement (Variables|Character|GetCharacterMovement))
  (bind _springarm (Variables|Default|GetSpringArm))
  (if (AI|Components|NavMovement|IsFalling _charactermovement)
    (Variables|/Script/Engine.SpringArmComponent|SetCameraLagSpeed _springarm (Math|Float|Lerp (Variables|/Script/Engine.SpringArmComponent|GetCameraLagSpeed _springarm) 0.0 Delta) :!label _label)
    (elif (> (Math|Vector|VectorLength (Variables|/Script/Engine.MovementComponent|GetVelocity _charactermovement)) 3e+02)
      (Variables|/Script/Engine.SpringArmComponent|SetCameraLagSpeed _springarm (Math|Float|Lerp (Variables|/Script/Engine.SpringArmComponent|GetCameraLagSpeed _springarm) 1.0 Delta))
      (else
        (goto _label)))))

(fn NewFunction0)